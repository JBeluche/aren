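; Story controller that runs a short scripted scene on BeginPlay between OldMan_1 and MainCharacter_1.
; After a brief delay it plays the main character's stand-up montage and sends the old man walking to them, then plays the montage again after a longer wait.
; Helpers resolve each character class to its first placed BP_CharacterBase instance and move it via its AI controller with SimpleMoveToActor.
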(event EventBeginPlay
  (Utilities|FlowControl|Delay 0.2)
  (CallFunction|Stupid)
  (CallFunction|MoveOneActortoOther "/Game/Characters/Generated/OldMan_1.OldMan_1_C" "/Game/Characters/Generated/MainCharacter_1.MainCharacter_1_C")
  (Utilities|FlowControl|Delay 5.0)
  (bind _character (CallFunction|GetCharacter "/Game/Characters/Generated/MainCharacter_1.MainCharacter_1_C"))
  (Animation|PlayAnimMontage _character "/Game/Characters/Modular/Animations/StandUp_Montage.StandUp_Montage" 1.0 "Default"))

(fn ConstructionScript)

(fn MoveOneActortoOther
  (params (Actor1 :type Actor%20Class%20Reference) (NewParam1 :type Actor%20Class%20Reference))
  (bind _character (CallFunction|GetCharacter NewParam1))
  (bind _character_2 (CallFunction|GetCharacter Actor1))
  (AI|Navigation|SimpleMovetoActor (AI|GetAIController _character_2) _character))

(fn GetCharacter
  (params (Actor :type Actor%20Class%20Reference))
  (bind _outactors (Actor|GetAllActorsOfClass Actor))
  (for _array_element _outactors
    (bind _asbp_character_base (Utilities|Casting|CastToBP_CharacterBase _array_element))
    (return _asbp_character_base)))

(fn Stupid
  (bind _character (CallFunction|GetCharacter "/Game/Characters/Generated/MainCharacter_1.MainCharacter_1_C"))
  (Utilities|FlowControl|DoOnce false
    (:Completed
      (Class|StoryControllerBase|PlayAnimationonCharacter _character "/Game/Characters/Modular/Animations/StandUp_Montage.StandUp_Montage" false))))